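; Player Blueprint for a runner, providing a cube roll during jumps and smooth sideways movement through two timeline-driven events.
; TriggerJumpTimeline plays the Rotation timeline, lerping the Cube's relative rotation from the actor's rotation to a quarter turn back in pitch.
; SetActorNewLocation, gated by CanMove, plays AddMovement to lerp actor Y toward a target.
; CanMove resets on timeline updates, not on completion.
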(event EventBeginPlay)

(event Collision|EventActorBeginOverlap
  (params (OtherActor :type Actor%20Object%20Reference)))

(event EventTick
  (params (DeltaSeconds :type Float%20%28single-precision%29)))

(event EventSetActorNewLocation
  (params (TargetYLocation :type Float%20%28single-precision%29))
  (bind _returnvalue (Transformation|GetActorLocation))
  ;[1 0.9953 0.7708] Timeline For Smooth Side Movement
  (if (Variables|Default|GetCanMove)
    (Variables|Default|SetCanMove false)
    (bind _moveactor (Timeline|AddMovement PlayFromStart)
      (:Update
        (Transformation|SetActorLocation (Math|Vector|MakeVector (.x _returnvalue) (Math|Float|Lerp (.y _returnvalue) TargetYLocation _moveactor) (.z _returnvalue)) false false)
        (Variables|Default|SetCanMove true)))))

(event EventTriggerJumpTimeline
  (bind _returnvalue (Transformation|GetActorRotation))
  (bind (_roll _pitch _yaw) (Math|Rotator|BreakRotator _returnvalue))
  ;[1 0.4479 0.7125] Timeline For Rolling The Cube While Jumping
  (bind _alpha_ (Timeline|Rotation PlayFromStart)
    (:Update
      (Transformation|SetRelativeRotation (Variables|Default|GetCube) (Math|Rotator|Lerp(Rotator) _returnvalue (Math|Rotator|MakeRotator _roll (+ _pitch -9e+01) _yaw) _alpha_) false false))))

(fn ConstructionScript)